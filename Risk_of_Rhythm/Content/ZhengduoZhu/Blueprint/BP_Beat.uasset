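; BP_Beat is a rhythm-game note that becomes a projectile attack when broken and hurts the player when missed.
; BreakBeat spawns a particle burst, then launches the note up or down by Direction with opposing gravity.
; The Credit rating scales damage and mana and grows the combo, or on Miss damages the player and resets it.
; DamageCollision damages overlapped actors; a dynamic plane material shows player health at spawn.
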(event OnComponentBeginOverlap(DamageCollision)
  (params (OverlappedComponent :type Primitive%20Component%20Object%20Reference) (OtherActor :type Actor%20Object%20Reference) (OtherComp :type Primitive%20Component%20Object%20Reference) (OtherBodyIndex :type Integer) (bFromSweep :type Boolean) (SweepResult :type Hit%20Result%20Structure%20%28by%20ref%29))
  (Game|Damage|ApplyDamage OtherActor (Variables|Default|GetDamage) 0 0))

(event Custom|Attack_U
  (bind _perfectmultiplier (Variables|Default|GetPerfectMultiplier))
  (bind _greatmultiplier (Variables|Default|GetGreatMultiplier))
  (bind _goodmultiplier (Variables|Default|GetGoodMultiplier))
  (bind _projectilemovement (Variables|Default|GetProjectileMovement))
  (Components|Movement|StopMovementImmediately _projectilemovement)
  (Variables|/Script/Engine.ProjectileMovementComponent|SetProjectileGravityScale _projectilemovement 2.0)
  (Variables|/Script/Engine.ProjectileMovementComponent|SetInitialSpeed _projectilemovement 0.0)
  (Variables|/Script/Engine.ProjectileMovementComponent|SetMaxSpeed _projectilemovement 0.0)
  (Variables|/Script/Engine.MovementComponent|SetVelocity _projectilemovement "0,1000.000000,700.000000")
  (switch string (Variables|Default|GetCredit)
    (:Perfect
      (Variables|Default|SetManaAmount (* (Variables|Default|GetNormalMana) _perfectmultiplier))
      (Variables|Default|SetDamage (* (Variables|Default|GetDamage) _perfectmultiplier))
      (bind _asversion_2_character (Utilities|Casting|CastToVersion2_Character (Game|GetPlayerCharacter 0) :!label _label))
      (Default|AddMana _asversion_2_character (Variables|Default|GetManaAmount))
      (Math|Integer|IncrementInt (Variables|/Game/ZhengduoZhu/Character/Version2_Character.Version2_Character_C|GetCombo _asversion_2_character)))
    (:Great
      (Variables|Default|SetManaAmount (* (Variables|Default|GetNormalMana) _greatmultiplier))
      (Variables|Default|SetDamage (* (Variables|Default|GetDamage) _greatmultiplier))
      (goto _label))
    (:Good
      (Variables|Default|SetManaAmount (* (Variables|Default|GetNormalMana) _goodmultiplier))
      (Variables|Default|SetDamage (* (Variables|Default|GetDamage) _goodmultiplier))
      (goto _label))
    (:Miss
      (Variables|Default|SetDamage (Variables|Default|GetNormalDamage))
      (bind _asversion_2_character_2 (Utilities|Casting|CastToVersion2_Character (Game|GetPlayerCharacter 0)))
      (Game|Damage|ApplyDamage _asversion_2_character_2 (Variables|Default|GetDamage) 0 0)
      (Variables|/Game/ZhengduoZhu/Character/Version2_Character.Version2_Character_C|SetCombo _asversion_2_character_2 0)
      (Actor|DestroyActor)
      (Development|PrintString (Utilities|String|ToString(Float) (Variables|/Game/ZhengduoZhu/Character/Version2_Character.Version2_Character_C|GetHealth _asversion_2_character_2))))))

(event Custom|Attack_D
  (bind _projectilemovement (Variables|Default|GetProjectileMovement))
  (bind _perfectmultiplier (Variables|Default|GetPerfectMultiplier))
  (bind _greatmultiplier (Variables|Default|GetGreatMultiplier))
  (bind _goodmultiplier (Variables|Default|GetGoodMultiplier))
  (Components|Movement|StopMovementImmediately _projectilemovement)
  (Variables|/Script/Engine.ProjectileMovementComponent|SetProjectileGravityScale _projectilemovement -2.0)
  (Variables|/Script/Engine.ProjectileMovementComponent|SetInitialSpeed _projectilemovement 0.0)
  (Variables|/Script/Engine.ProjectileMovementComponent|SetMaxSpeed _projectilemovement 0.0)
  (Variables|/Script/Engine.MovementComponent|SetVelocity _projectilemovement "0,1000.000000,-700.000000")
  (switch string (Variables|Default|GetCredit)
    (:Perfect
      (Variables|Default|SetManaAmount (* (Variables|Default|GetNormalMana) _perfectmultiplier))
      (Variables|Default|SetDamage (* (Variables|Default|GetDamage) _perfectmultiplier))
      (bind _asversion_2_character (Utilities|Casting|CastToVersion2_Character (Game|GetPlayerCharacter 0) :!label _label))
      (Default|AddMana _asversion_2_character (Variables|Default|GetManaAmount))
      (Math|Integer|IncrementInt (Variables|/Game/ZhengduoZhu/Character/Version2_Character.Version2_Character_C|GetCombo _asversion_2_character)))
    (:Great
      (Variables|Default|SetManaAmount (* (Variables|Default|GetNormalMana) _greatmultiplier))
      (Variables|Default|SetDamage (* (Variables|Default|GetDamage) _greatmultiplier))
      (goto _label))
    (:Good
      (Variables|Default|SetManaAmount (* (Variables|Default|GetNormalMana) _goodmultiplier))
      (Variables|Default|SetDamage (* (Variables|Default|GetDamage) _goodmultiplier))
      (goto _label))
    (:Miss
      (Variables|Default|SetDamage (Variables|Default|GetNormalDamage))
      (bind _asversion_2_character_2 (Utilities|Casting|CastToVersion2_Character (Game|GetPlayerCharacter 0)))
      (Game|Damage|ApplyDamage _asversion_2_character_2 (Variables|Default|GetDamage) 0 0)
      (Variables|/Game/ZhengduoZhu/Character/Version2_Character.Version2_Character_C|SetCombo _asversion_2_character_2 0)
      (Actor|DestroyActor)
      (Development|PrintString (Utilities|String|ToString(Float) (Variables|/Game/ZhengduoZhu/Character/Version2_Character.Version2_Character_C|GetHealth _asversion_2_character_2))))))

(event Custom|Attack
  (switch string (Variables|Default|GetDirection)
    (:UP
      (CallFunction|AttackU))
    (:DOWN
      (CallFunction|AttackD))))

(event EventBeginPlay
  (bind _returnvalue (Rendering|Material|CreateDynamicMaterialInstance (Variables|Default|GetPlane) 0 "/Game/ZhengduoZhu/Material/MI_Health.MI_Health" "None" :!class /Script/Engine.PrimitiveComponent))
  (bind _asversion_2_character (Utilities|Casting|CastToVersion2_Character (Game|GetPlayerCharacter 0)))
  (Rendering|Material|SetScalarParameterValue _returnvalue "Percentage" (/ (Variables|/Game/ZhengduoZhu/Character/Version2_Character.Version2_Character_C|GetHealth _asversion_2_character) (Variables|/Game/ZhengduoZhu/Character/Version2_Character.Version2_Character_C|GetMaxHealth _asversion_2_character)) :!class /Script/Engine.MaterialInstanceDynamic)
  (Rendering|Material|SetVectorParameterValue _returnvalue "LiquidColor" (Utilities|Struct|MakeLinearColor (* (- 1.0 (/ (Variables|/Game/ZhengduoZhu/Character/Version2_Character.Version2_Character_C|GetHealth _asversion_2_character) (Variables|/Game/ZhengduoZhu/Character/Version2_Character.Version2_Character_C|GetMaxHealth _asversion_2_character))) 2e+02) (* (/ (Variables|/Game/ZhengduoZhu/Character/Version2_Character.Version2_Character_C|GetHealth _asversion_2_character) (Variables|/Game/ZhengduoZhu/Character/Version2_Character.Version2_Character_C|GetMaxHealth _asversion_2_character)) 2e+02) 0.0 0.0) :!class /Script/Engine.MaterialInstanceDynamic))

(event Collision|EventActorBeginOverlap
  (params (OtherActor :type Actor%20Object%20Reference)))

(event EventTick
  (params (DeltaSeconds :type Float%20%28single-precision%29)))

(fn ConstructionScript)

(fn BreakBeat
  (Effects|SpawnEmitteratLocation "/Game/ZhengduoZhu/Particle/P_BreakNote.P_BreakNote" (Transformation|GetActorLocation) "0, 0, 0" "0.300000,0.300000,0.300000")
  (CallFunction|Attack))

(fn Miss
  (Game|Damage|ApplyDamage (Game|Player|GetPlayerPawn 0) (Variables|Default|GetDamage) 0 0)
  (Actor|DestroyActor))