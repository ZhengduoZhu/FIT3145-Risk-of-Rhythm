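; BP_Monster is an enemy that starts a battle through GM_Zheng when the player character enters its sphere, then teleports to a hardcoded battle position.
; Incoming damage is scaled by DEF, updates its widget health bar, and reports a win to the game mode at zero health.
; Once StartBattle runs, a looping timer checks attack progress, raised by IncreaseProgress, and damages the player with ATK when full.
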(event OnComponentBeginOverlap(Sphere)
  (params (OverlappedComponent :type Primitive%20Component%20Object%20Reference) (OtherActor :type Actor%20Object%20Reference) (OtherComp :type Primitive%20Component%20Object%20Reference) (OtherBodyIndex :type Integer) (bFromSweep :type Boolean) (SweepResult :type Hit%20Result%20Structure%20%28by%20ref%29))
  (bind _mygamemode (Variables|Default|GetMyGameMode))
  (Utilities|Casting|CastToZheng_Character OtherActor
    (:then
      (Utilities|IsValid _mygamemode
        (:Is%20Valid
          (Default|StartBattle _mygamemode self)
          (Transformation|SetActorTransform (Math|Transform|MakeTransform "-30.000000,11080.000000,-160.000000" "0,-90.000000, 0" "1,1,1")))
        (:Is%20Not%20Valid
          (Development|PrintString "Gamemode is not Valid"))))
    (:CastFailed
      (Development|PrintString "CastCharacterFailed!"))))

(event Custom|StartBattle
  (Utilities|Time|SetTimerbyEvent (delegate Custom|Check) 0.2 true))

(event Custom|Attack
  (Game|Damage|ApplyDamage (Game|GetPlayerCharacter 0) (Variables|State|GetATK) 0 0))

(event Custom|Check
  (if (>= (Variables|State|GetAttackProgress) (Variables|State|GetMaxAttackProgress))
    (Variables|State|SetAttackProgress 0.0)
    (CallFunction|Attack)))

(event Custom|IncreaseProgress
  (Variables|State|SetAttackProgress (Math|Float|Clamp(Float) (+ (Variables|State|GetAttackProgress) 4e+01) 0.0 (Variables|State|GetMaxAttackProgress))))

(event EventBeginPlay
  (bind _asgm_zheng (Utilities|Casting|CastToGM_Zheng (Game|GetGameMode)))
  (Variables|Default|SetMyGameMode _asgm_zheng)
  (bind _asenemy_health_bar (Utilities|Casting|CastToEnemyHealthBar (UserInterface|GetUserWidgetObject (Variables|Default|GetHealthBar))))
  (Variables|Default|SetMyHealthBar _asenemy_health_bar)
  (bind _asenemy_progress_bar (Utilities|Casting|CastToEnemyProgressBar (UserInterface|GetUserWidgetObject (Variables|Default|GetAttackProgressBar))))
  (bind _output_get (Variables|Default|SetMyProgressBar _asenemy_progress_bar))
  (Variables|/Game/ZhengduoZhu/UI/EnemyProgressBar.EnemyProgressBar_C|SetOwningCharacter _output_get self))

(event Collision|EventActorBeginOverlap
  (params (OtherActor :type Actor%20Object%20Reference)))

(event EventTick
  (params (DeltaSeconds :type Float%20%28single-precision%29)))

(event Game|Damage|EventAnyDamage
  (params (Damage :type Float%20%28single-precision%29) (DamageType :type Damage%20Type%20Object%20Reference) (InstigatedBy :type Controller%20Object%20Reference) (DamageCauser :type Actor%20Object%20Reference))
  (Variables|State|SetHealth (- (Variables|State|GetHealth) (* Damage (Variables|State|GetDEF))))
  (Default|SetPercentage (Variables|Default|GetMyHealthBar) (/ (Variables|State|GetHealth) (Variables|State|GetMaxHealth)))
  (if (<= (Variables|State|GetHealth) 0.0)
    (Default|WinBattle (Variables|Default|GetMyGameMode))))

(fn ConstructionScript)