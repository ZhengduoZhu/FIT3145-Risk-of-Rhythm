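; Rhythm-game beat spawner and hit-judgement zone for the Zheng game mode.
; AutoSpawnBeat starts a looping timer at the game mode's BPM that spawns scaled-down BP_Beat actors at SpawnPoint.
; Overlaps with nested Perfect, Great and Good components set each beat's Credit, downgrading on exit to Miss.
; The Good zone also adds and removes beats in the game mode's Notes and triggers its input validity check.
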(event OnComponentBeginOverlap(Perfect)
  (params (OverlappedComponent :type Primitive%20Component%20Object%20Reference) (OtherActor :type Actor%20Object%20Reference) (OtherComp :type Primitive%20Component%20Object%20Reference) (OtherBodyIndex :type Integer) (bFromSweep :type Boolean) (SweepResult :type Hit%20Result%20Structure%20%28by%20ref%29))
  (bind _asbp_beat (Utilities|Casting|CastToBP_Beat OtherActor))
  (Variables|/Game/ZhengduoZhu/Blueprint/BP_Beat.BP_Beat_C|SetCredit _asbp_beat "Perfect"))

(event OnComponentEndOverlap(Perfect)
  (params (OverlappedComponent :type Primitive%20Component%20Object%20Reference) (OtherActor :type Actor%20Object%20Reference) (OtherComp :type Primitive%20Component%20Object%20Reference) (OtherBodyIndex :type Integer))
  (bind _asbp_beat (Utilities|Casting|CastToBP_Beat OtherActor))
  (Variables|/Game/ZhengduoZhu/Blueprint/BP_Beat.BP_Beat_C|SetCredit _asbp_beat "Great"))

(event OnComponentBeginOverlap(Great)
  (params (OverlappedComponent :type Primitive%20Component%20Object%20Reference) (OtherActor :type Actor%20Object%20Reference) (OtherComp :type Primitive%20Component%20Object%20Reference) (OtherBodyIndex :type Integer) (bFromSweep :type Boolean) (SweepResult :type Hit%20Result%20Structure%20%28by%20ref%29))
  (bind _asbp_beat (Utilities|Casting|CastToBP_Beat OtherActor))
  (Variables|/Game/ZhengduoZhu/Blueprint/BP_Beat.BP_Beat_C|SetCredit _asbp_beat "Great"))

(event OnComponentEndOverlap(Great)
  (params (OverlappedComponent :type Primitive%20Component%20Object%20Reference) (OtherActor :type Actor%20Object%20Reference) (OtherComp :type Primitive%20Component%20Object%20Reference) (OtherBodyIndex :type Integer))
  (bind _asbp_beat (Utilities|Casting|CastToBP_Beat OtherActor))
  (Variables|/Game/ZhengduoZhu/Blueprint/BP_Beat.BP_Beat_C|SetCredit _asbp_beat "Good"))

(event OnComponentBeginOverlap(Good)
  (params (OverlappedComponent :type Primitive%20Component%20Object%20Reference) (OtherActor :type Actor%20Object%20Reference) (OtherComp :type Primitive%20Component%20Object%20Reference) (OtherBodyIndex :type Integer) (bFromSweep :type Boolean) (SweepResult :type Hit%20Result%20Structure%20%28by%20ref%29))
  (Variables|/Game/ZhengduoZhu/Blueprint/GM_Zheng.GM_Zheng_C|SetValidInput (Variables|Default|GetMyGameMode) false)
  (bind _asbp_beat (Utilities|Casting|CastToBP_Beat OtherActor))
  (Utilities|Array|Add (Variables|/Game/ZhengduoZhu/Blueprint/GM_Zheng.GM_Zheng_C|GetNotes (Variables|Default|GetMyGameMode)) _asbp_beat)
  (Variables|/Game/ZhengduoZhu/Blueprint/BP_Beat.BP_Beat_C|SetCredit _asbp_beat "Good"))

(event OnComponentEndOverlap(Good)
  (params (OverlappedComponent :type Primitive%20Component%20Object%20Reference) (OtherActor :type Actor%20Object%20Reference) (OtherComp :type Primitive%20Component%20Object%20Reference) (OtherBodyIndex :type Integer))
  (bind _asbp_beat (Utilities|Casting|CastToBP_Beat OtherActor))
  (Utilities|Array|RemoveItem (Variables|/Game/ZhengduoZhu/Blueprint/GM_Zheng.GM_Zheng_C|GetNotes (Variables|Default|GetMyGameMode)) _asbp_beat)
  (Variables|/Game/ZhengduoZhu/Blueprint/BP_Beat.BP_Beat_C|SetCredit _asbp_beat "Miss")
  (Default|CheckValidInput (Variables|Default|GetMyGameMode)))

(event Custom|SpawnBeat
  (bind _spawnpoint (Variables|Default|GetSpawnPoint))
  (bind _returnvalue (Transformation|GetWorldTransform _spawnpoint))
  (Game|SpawnActorfromClass "/Game/ZhengduoZhu/Blueprint/BP_Beat.BP_Beat_C" (Math|Transform|MakeTransform (.location _returnvalue) (.rotation _returnvalue) "0.100000,0.100000,0.100000") "Undefined" 0 0))

(event Custom|AutoSpawnBeat
  (Utilities|Time|SetTimerbyEvent (delegate Custom|SpawnBeat) (/ 6e+01 (Variables|/Game/ZhengduoZhu/Blueprint/GM_Zheng.GM_Zheng_C|GetBPM (Variables|Default|GetMyGameMode))) true))

(event EventBeginPlay
  (bind _asgm_zheng (Utilities|Casting|CastToGM_Zheng (Game|GetGameMode)))
  (Variables|Default|SetMyGameMode _asgm_zheng))

(event Collision|EventActorBeginOverlap
  (params (OtherActor :type Actor%20Object%20Reference)))

(event EventTick
  (params (DeltaSeconds :type Float%20%28single-precision%29)))

(fn ConstructionScript)