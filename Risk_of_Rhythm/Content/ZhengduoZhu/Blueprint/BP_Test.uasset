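; BP_Test is a test spawner actor that launches a scaled-down BP_TestBeats projectile from its own location every second on a looping timer.
; Each projectile gets a random gravity scale, negative or positive, so gravity can pull it up or down.
; Its launch velocity has fixed horizontal components and a vertical component derived from Gravity and that random scale, so the vertical arc varies per shot.
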(event Custom|Spawn
  (bind _returnvalue (Game|SpawnActorfromClass "/Game/ZhengduoZhu/Blueprint/BP_TestBeats.BP_TestBeats_C" (Math|Transform|MakeTransform (Transformation|GetActorLocation) "0, 0, 0" "0.200000,0.200000,0.200000") "Undefined" 0 0))
  (bind _output_get (Variables|Default|SetGravityScale (Math|Random|RandomFloatinRange -1.0 1.0)))
  (Variables|/Script/Engine.ProjectileMovementComponent|SetProjectileGravityScale (Variables|/Game/ZhengduoZhu/Blueprint/BP_TestBeats.BP_TestBeats_C|GetProjectileMovement _returnvalue) _output_get)
  (Variables|Default|SetZ_Velocity (* (Variables|Default|GetGravity) (Variables|Default|GetGravityScale) 0.5))
  (Variables|/Script/Engine.MovementComponent|SetVelocity (Variables|/Game/ZhengduoZhu/Blueprint/BP_TestBeats.BP_TestBeats_C|GetProjectileMovement _returnvalue) (Math|Vector|MakeVector -1e+02 1e+02 (Variables|Default|GetZ_Velocity))))

(event EventBeginPlay
  (Utilities|Time|SetTimerbyEvent (delegate Custom|Spawn) 1.0 true))

(event Collision|EventActorBeginOverlap
  (params (OtherActor :type Actor%20Object%20Reference)))

(event EventTick
  (params (DeltaSeconds :type Float%20%28single-precision%29)))

(fn ConstructionScript)