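; GM_Zheng is a game mode that runs a rhythm-based battle, moving from camera fade and countdown into a level sequence.
; Key presses are graded Perfect, Great, Good or Miss from timing-window flags, with combo popups for feedback.
; Valid keys build a sequence matched against skill patterns at the beat count: Attack damages the monster, Defence only prints, and misses clear it.
; A BPM-driven looping timer plays the drum beat.
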(event Custom|StartBattle
  (params (Monster :type BP%20Monster%20Object%20Reference))
  (bind _mycharacter (Variables|Default|GetMyCharacter))
  ;[1 1 1] Start Battle
  (Transformation|SetActorTransform _mycharacter (Math|Transform|MakeTransform "-40.000000,10490.000000,-160.000000" "0,90.000000, 0" "1,1,1"))
  (Class|NavMovementComponent|StopActiveMovement (Variables|/Script/Engine.Character|GetCharacterMovement _mycharacter))
  (Variables|Default|SetMyMonster Monster)
  (Variables|/Game/ZhengduoZhu/Blueprint/PC_Zheng.PC_Zheng_C|SetBattleMode (Variables|Default|GetMyPlayerController) true)
  (Variables|/Game/ZhengduoZhu/Character/Zheng_Character.Zheng_Character_C|SetBattleMode (Variables|Default|GetMyCharacter) true)
  (Variables|/Script/Engine.PlayerController|SetbShowMouseCursor (Game|GetPlayerController 0) false)
  (CameraFades|StartCameraFade :self (Game|GetPlayerCameraManager 0) :ToAlpha 1.0 :Duration 1.0 :bHoldWhenFinished true)
  (Utilities|FlowControl|Delay 1.0)
  (Game|Player|SetViewTargetwithBlend (Game|GetPlayerController 0) (Variables|Default|GetBattleCamera) 0.0 "VTBlend_EaseInOut" 0.0 false)
  (CameraFades|StartCameraFade :self (Game|GetPlayerCameraManager 0) :FromAlpha 1.0 :Duration 1.0 :bHoldWhenFinished true)
  (UserInterface|Viewport|AddtoViewport (Variables|Default|GetMyBattleUI) 0)
  (bind _returnvalue (UserInterface|CreateWidget "/Game/ZhengduoZhu/UI/CountDownUI.CountDownUI_C" (Variables|Default|GetMyPlayerController)))
  (UserInterface|Viewport|AddtoViewport _returnvalue 0)
  (Utilities|FlowControl|Delay 5.0)
  (Widget|RemovefromParent _returnvalue)
  (Sequencer|Player|Play (Variables|Default|GetTestSequencer) :!class /Script/MovieScene.MovieSceneSequencePlayer))

(event Custom|Input
  (params (InputKey :type String))
  (bind _inputsequence (Variables|Battle|GetInputSequence))
  ;[1 1 1] Receive Input
  (if (Variables|Default|GetBattleStart)
    (if (Variables|Matching|GetPerfectOpen)
      (Development|PrintString "Perfect!")
      (Variables|Matching|SetValidInput true)
      (CallFunction|CreateComboUI "Perfect!")
      (Utilities|Array|Add _inputsequence InputKey :!label _label)
      (Default|DetectedInput (Variables|Default|GetMyBattleUI) InputKey)
      (if (>= (Utilities|Array|Length _inputsequence) (Variables|Battle|GetBattleBeats))
        (CallFunction|MatchingSkill))
      (elif (Variables|Matching|GetGreatOpen)
        (Development|PrintString "Great!")
        (Variables|Matching|SetValidInput true)
        (CallFunction|CreateComboUI "Great!")
        (goto _label)
        (elif (Variables|Matching|GetGoodOpen)
          (Development|PrintString "Good!")
          (Variables|Matching|SetValidInput true)
          (CallFunction|CreateComboUI "Good!")
          (goto _label)
          (else
            (Variables|Matching|SetValidInput false)
            (CallFunction|ErrorInput)
            (CallFunction|CreateComboUI "Miss!")))))))

(event Custom|CreateBeats
  (Utilities|Time|SetTimerbyFunctionName 0 "TriggerBeats" (/ 6e+01 (Variables|Default|GetBPM)) true))

(event Custom|CheckValidInput
  ;[1 1 1] Check Input
  (if (not (Variables|Matching|GetValidInput))
    (CallFunction|ErrorInput)))

(event Custom|ErrorInput
  ;[1 1 1] Error Input
  (Development|PrintString "Miss!")
  (Utilities|Array|Clear (Variables|Battle|GetInputSequence))
  (Default|RefreshInput (Variables|Default|GetMyBattleUI))
  (CallFunction|CreateComboUI "Miss!"))

(event Custom|MatchingSkill
  (bind _skillgroup (Variables|Battle|GetSkillGroup))
  (bind _inputsequence (Variables|Battle|GetInputSequence))
  ;[1 1 1] Matching Skill
  (if (Utilities|Array|Identical (.attack _skillgroup) _inputsequence)
    (Development|PrintString "Attack")
    (CallFunction|DealingDamage)
    (elif (Utilities|Array|Identical _inputsequence (.defence _skillgroup))
      (Development|PrintString "Defence")
      (else
        (Development|PrintString "No Matching!"))))
  (Utilities|Array|Clear (Variables|Battle|GetInputSequence))
  (Default|RefreshInput (Variables|Default|GetMyBattleUI)))

(event Custom|CreateComboUI
  (params (Input :type Text))
  ;[1 1 1] Create Combo UI
  (bind _returnvalue (UserInterface|CreateWidget "/Game/ZhengduoZhu/UI/ComboWidget.ComboWidget_C" (Variables|Default|GetMyPlayerController)))
  (Default|SetComboText _returnvalue Input)
  (UserInterface|Viewport|AddtoViewport _returnvalue 0))

(event Custom|Dealing%20Damage
  ;[1 1 1] Dealing Damage
  (Game|Damage|ApplyDamage (Variables|Default|GetMyMonster) (* (Variables|/Game/ZhengduoZhu/Character/Zheng_Character.Zheng_Character_C|GetATK (Variables|Default|GetMyCharacter)) (Variables|Battle|GetDamageRatio)) 0 0))

(event Custom|WinBattle
  ;[1 1 1] Win
  (Development|PrintString "You Win")
  (Game|SetGamePaused true))

(event EventBeginPlay
  ;[1 1 1] Initialize
  (Variables|Default|SetBattleCamera (Components|GetOwner (Variables|Default|GetCamera)))
  (bind _aspc_zheng (Utilities|Casting|CastToPC_Zheng (Game|GetPlayerController 0)))
  (bind _output_get (Variables|Default|SetMyPlayerController _aspc_zheng))
  (bind _aszheng_character (Utilities|Casting|CastToZheng_Character (Pawn|GetControlledPawn _output_get)))
  (Variables|Default|SetMyCharacter _aszheng_character)
  (Transformation|SetActorTransform (Variables|Default|GetBattleCamera) (Math|Transform|MakeTransform "-600.000000,10790.000000,-130.000000" "-10.000000, 0, 0" "1,1,1"))
  (bind _returnvalue (UserInterface|CreateWidget "/Game/ZhengduoZhu/UI/BattleUI.BattleUI_C" (Variables|Default|GetMyPlayerController)))
  (Variables|Default|SetMyBattleUI _returnvalue)
  (bind _returnvalue_2 (Sequencer|Player|CreateLevelSequencePlayer "/Game/ZhengduoZhu/TestSequencer.TestSequencer"))
  (Variables|Default|SetTestSequencer _returnvalue_2))

(fn ConstructionScript)

(fn TriggerBeats
  (Audio|PlaySound2D "/Game/ZhengduoZhu/Audio/Drum.Drum" 1.0 1.0 0.0 0 0))