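; Background actor that recolors its two meshes to match the player character's Mana tier.
; BeginPlay caches the character and creates dynamic material instances for both meshes.
; Tick checks Mana against 90/60/30 thresholds, using DoOnce gates that reset one another so each tier change fires once.
; Tier events run timelines that blend the "Effect" parameter from its current color to red, blue, yellow or black.
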(event Custom|Set%200
  (bind _mi00 (Variables|Default|GetMI00))
  (bind _mi01 (Variables|Default|GetMI01))
  (Utilities|FlowControl|Sequence
    (:then_0
      (bind _returnvalue (Rendering|Material|GetVectorParameterValue _mi00 "Effect" :!class /Script/Engine.MaterialInstanceDynamic))
      (bind _newtrack_0 (Timeline|Timeline_0 PlayFromStart)
        (:Update
          (Rendering|Material|SetVectorParameterValue _mi00 "Effect" (Math|Color|Lerp(LinearColor) _returnvalue "(R=0.000000,G=0.000000,B=0.000000,A=1.000000)" _newtrack_0) :!class /Script/Engine.MaterialInstanceDynamic))))
    (:then_1
      (bind _returnvalue_2 (Rendering|Material|GetVectorParameterValue _mi01 "Effect" :!class /Script/Engine.MaterialInstanceDynamic))
      (bind _newtrack_0_2 (Timeline|Timeline_1 PlayFromStart)
        (:Update
          (Rendering|Material|SetVectorParameterValue _mi01 "Effect" (Math|Color|Lerp(LinearColor) _returnvalue_2 "(R=0.000000,G=0.000000,B=0.000000,A=1.000000)" _newtrack_0_2) :!class /Script/Engine.MaterialInstanceDynamic))))))

(event Custom|Set%2030
  (bind _mi00 (Variables|Default|GetMI00))
  (bind _mi01 (Variables|Default|GetMI01))
  (Utilities|FlowControl|Sequence
    (:then_0
      (bind _returnvalue (Rendering|Material|GetVectorParameterValue _mi00 "Effect" :!class /Script/Engine.MaterialInstanceDynamic))
      (bind _newtrack_0 (Timeline|Lerp PlayFromStart)
        (:Update
          (Rendering|Material|SetVectorParameterValue _mi00 "Effect" (Math|Color|Lerp(LinearColor) _returnvalue "(R=0.979167,G=0.840020,B=0.036154,A=1.000000)" _newtrack_0) :!class /Script/Engine.MaterialInstanceDynamic))))
    (:then_1
      (bind _returnvalue_2 (Rendering|Material|GetVectorParameterValue _mi01 "Effect" :!class /Script/Engine.MaterialInstanceDynamic))
      (bind _newtrack_0_2 (Timeline|Lerp2 PlayFromStart)
        (:Update
          (Rendering|Material|SetVectorParameterValue _mi01 "Effect" (Math|Color|Lerp(LinearColor) _returnvalue_2 "(R=0.979167,G=0.840020,B=0.036154,A=1.000000)" _newtrack_0_2) :!class /Script/Engine.MaterialInstanceDynamic))))))

(event Custom|Set%2060
  (bind _mi00 (Variables|Default|GetMI00))
  (bind _mi01 (Variables|Default|GetMI01))
  (Utilities|FlowControl|Sequence
    (:then_0
      (bind _returnvalue (Rendering|Material|GetVectorParameterValue _mi00 "Effect" :!class /Script/Engine.MaterialInstanceDynamic))
      (bind _newtrack_0 (Timeline|Timeline_2 PlayFromStart)
        (:Update
          (Rendering|Material|SetVectorParameterValue _mi00 "Effect" (Math|Color|Lerp(LinearColor) _returnvalue "(R=0.055999,G=0.286791,B=0.979167,A=1.000000)" _newtrack_0) :!class /Script/Engine.MaterialInstanceDynamic))))
    (:then_1
      (bind _returnvalue_2 (Rendering|Material|GetVectorParameterValue _mi01 "Effect" :!class /Script/Engine.MaterialInstanceDynamic))
      (bind _newtrack_0_2 (Timeline|Timeline_3 PlayFromStart)
        (:Update
          (Rendering|Material|SetVectorParameterValue _mi01 "Effect" (Math|Color|Lerp(LinearColor) _returnvalue_2 "(R=0.054198,G=0.340573,B=0.979167,A=1.000000)" _newtrack_0_2) :!class /Script/Engine.MaterialInstanceDynamic))))))

(event Custom|Set%2090
  (bind _mi00 (Variables|Default|GetMI00))
  (bind _mi01 (Variables|Default|GetMI01))
  (Utilities|FlowControl|Sequence
    (:then_0
      (bind _returnvalue (Rendering|Material|GetVectorParameterValue _mi00 "Effect" :!class /Script/Engine.MaterialInstanceDynamic))
      (bind _newtrack_0 (Timeline|Timeline_4 PlayFromStart)
        (:Update
          (Rendering|Material|SetVectorParameterValue _mi00 "Effect" (Math|Color|Lerp(LinearColor) _returnvalue "(R=0.979167,G=0.072479,B=0.000000,A=1.000000)" _newtrack_0) :!class /Script/Engine.MaterialInstanceDynamic))))
    (:then_1
      (bind _returnvalue_2 (Rendering|Material|GetVectorParameterValue _mi01 "Effect" :!class /Script/Engine.MaterialInstanceDynamic))
      (bind _newtrack_0_2 (Timeline|Timeline_5 PlayFromStart)
        (:Update
          (Rendering|Material|SetVectorParameterValue _mi01 "Effect" (Math|Color|Lerp(LinearColor) _returnvalue_2 "(R=0.979167,G=0.027765,B=0.000000,A=1.000000)" _newtrack_0_2) :!class /Script/Engine.MaterialInstanceDynamic))))))

(event EventBeginPlay
  (bind _asversion_2_character (Utilities|Casting|CastToVersion2_Character (Game|GetPlayerCharacter 0)))
  (Variables|Default|SetMyCharacter _asversion_2_character)
  (bind _returnvalue (Rendering|Material|CreateDynamicMaterialInstance (Variables|Default|GetStaticMeshComponent0) 0 "/Game/ZhengduoZhu/Material/MI_Background.MI_Background" "None" :!class /Script/Engine.PrimitiveComponent))
  (Variables|Default|SetMI00 _returnvalue)
  (bind _returnvalue_2 (Rendering|Material|CreateDynamicMaterialInstance (Variables|Default|GetStaticMeshComponent1) 0 "/Game/ZhengduoZhu/Material/MI_Background1.MI_Background1" "None" :!class /Script/Engine.PrimitiveComponent))
  (Variables|Default|SetMI01 _returnvalue_2))

(event EventTick
  (params (DeltaSeconds :type Float%20%28single-precision%29))
  (bind _mycharacter (Variables|Default|GetMyCharacter))
  (bind _mana (Variables|/Game/ZhengduoZhu/Character/Version2_Character.Version2_Character_C|GetMana _mycharacter))
  (if (>= _mana 9e+01)
    (Utilities|FlowControl|DoOnce false :!label _label
      (:Completed
        (CallFunction|Set90)
        (Utilities|FlowControl|Sequence
          (:then_0
            (goto _label_2 Reset))
          (:then_1
            (goto _label_3 Reset))
          (:then_2
            (goto _label_4 Reset)))))
    (elif (>= _mana 6e+01)
      (Utilities|FlowControl|DoOnce false :!label _label_2
        (:Completed
          (CallFunction|Set60)
          (Utilities|FlowControl|Sequence
            (:then_0
              (goto _label Reset))
            (:then_1
              (goto _label_3 Reset))
            (:then_2
              (goto _label_4 Reset)))))
      (elif (>= _mana 3e+01)
        (Utilities|FlowControl|DoOnce false :!label _label_3
          (:Completed
            (CallFunction|Set30)
            (Utilities|FlowControl|Sequence
              (:then_0
                (goto _label Reset))
              (:then_1
                (goto _label_2 Reset))
              (:then_2
                (goto _label_4 Reset)))))
        (else
          (Utilities|FlowControl|DoOnce false :!label _label_4
            (:Completed
              (CallFunction|Set0)
              (Utilities|FlowControl|Sequence
                (:then_0
                  (goto _label Reset))
                (:then_1
                  (goto _label_2 Reset))
                (:then_2
                  (goto _label_3 Reset))))))))))

(fn ConstructionScript)

(fn Set90%
  (bind _returnvalue (Rendering|Material|CreateDynamicMaterialInstance (Variables|Default|GetStaticMeshComponent0) 0 "/Game/ZhengduoZhu/Material/MI_Background.MI_Background" "None" :!class /Script/Engine.PrimitiveComponent))
  (Rendering|Material|SetVectorParameterValue _returnvalue "Effect" "(R=1.000000,G=0.038897,B=0.108593,A=1.000000)" :!class /Script/Engine.MaterialInstanceDynamic)
  (bind _returnvalue_2 (Rendering|Material|CreateDynamicMaterialInstance (Variables|Default|GetStaticMeshComponent1) 0 "/Game/ZhengduoZhu/Material/MI_Background1.MI_Background1" "None" :!class /Script/Engine.PrimitiveComponent))
  (Rendering|Material|SetVectorParameterValue _returnvalue_2 "Effect" "(R=1.000000,G=0.038897,B=0.108593,A=1.000000)" :!class /Script/Engine.MaterialInstanceDynamic))

(fn Set60%
  (bind _returnvalue (Rendering|Material|CreateDynamicMaterialInstance (Variables|Default|GetStaticMeshComponent0) 0 "/Game/ZhengduoZhu/Material/MI_Background.MI_Background" "None" :!class /Script/Engine.PrimitiveComponent))
  (Rendering|Material|SetVectorParameterValue _returnvalue "Effect" "(R=0.082484,G=0.000000,B=1.000000,A=1.000000)" :!class /Script/Engine.MaterialInstanceDynamic)
  (bind _returnvalue_2 (Rendering|Material|CreateDynamicMaterialInstance (Variables|Default|GetStaticMeshComponent1) 0 "/Game/ZhengduoZhu/Material/MI_Background1.MI_Background1" "None" :!class /Script/Engine.PrimitiveComponent))
  (Rendering|Material|SetVectorParameterValue _returnvalue_2 "Effect" "(R=0.082484,G=0.000000,B=1.000000,A=1.000000)" :!class /Script/Engine.MaterialInstanceDynamic))

(fn Set30%
  (bind _returnvalue (Rendering|Material|CreateDynamicMaterialInstance (Variables|Default|GetStaticMeshComponent0) 0 "/Game/ZhengduoZhu/Material/MI_Background.MI_Background" "None" :!class /Script/Engine.PrimitiveComponent))
  (bind _returnvalue_2 (Rendering|Material|GetVectorParameterValue _returnvalue "Effect" :!class /Script/Engine.MaterialInstanceDynamic))
  (Rendering|Material|SetVectorParameterValue _returnvalue "Effect" (Math|Color|Lerp(LinearColor) :A _returnvalue_2) :!class /Script/Engine.MaterialInstanceDynamic)
  (bind _returnvalue_3 (Rendering|Material|CreateDynamicMaterialInstance (Variables|Default|GetStaticMeshComponent1) 0 "/Game/ZhengduoZhu/Material/MI_Background1.MI_Background1" "None" :!class /Script/Engine.PrimitiveComponent))
  (Rendering|Material|GetVectorParameterValue _returnvalue_3 "Effect" :!class /Script/Engine.MaterialInstanceDynamic)
  (Rendering|Material|SetVectorParameterValue :self _returnvalue_3 :ParameterName "Effect" :!class /Script/Engine.MaterialInstanceDynamic))

(fn Set0%
  (bind _returnvalue (Rendering|Material|CreateDynamicMaterialInstance (Variables|Default|GetStaticMeshComponent0) 0 "/Game/ZhengduoZhu/Material/MI_Background.MI_Background" "None" :!class /Script/Engine.PrimitiveComponent))
  (Rendering|Material|SetVectorParameterValue _returnvalue "Effect" "(R=0.000000,G=0.000000,B=0.000000,A=1.000000)" :!class /Script/Engine.MaterialInstanceDynamic)
  (bind _returnvalue_2 (Rendering|Material|CreateDynamicMaterialInstance (Variables|Default|GetStaticMeshComponent1) 0 "/Game/ZhengduoZhu/Material/MI_Background1.MI_Background1" "None" :!class /Script/Engine.PrimitiveComponent))
  (Rendering|Material|SetVectorParameterValue _returnvalue_2 "Effect" "(R=0.000000,G=0.000000,B=0.000000,A=1.000000)" :!class /Script/Engine.MaterialInstanceDynamic))