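; BP_MonsterVersion2 is an enemy monster that starts a battle when the player character enters its sphere.
; On overlap it passes itself to Version2_GM's StartBattle and teleports to a hardcoded location and rotation.
; Incoming damage is divided by DEF, subtracted from Health and shown on its health bar widget, and reaching zero calls the game mode's Win.
; BeginPlay also creates a level sequence player, which this graph never plays.
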(event OnComponentBeginOverlap(Sphere)
  (params (OverlappedComponent :type Primitive%20Component%20Object%20Reference) (OtherActor :type Actor%20Object%20Reference) (OtherComp :type Primitive%20Component%20Object%20Reference) (OtherBodyIndex :type Integer) (bFromSweep :type Boolean) (SweepResult :type Hit%20Result%20Structure%20%28by%20ref%29))
  (Utilities|Casting|CastToVersion2_Character OtherActor)
  (Utilities|IsValid (Variables|Default|GetMyGameMode)
    (:Is%20Valid
      (Default|StartBattle (Variables|Default|GetMyGameMode) self)
      (Transformation|SetActorTransform (Math|Transform|MakeTransform "-676.000000,9923.000000,250.000000" "0,-90.000000, 0" "1,1,1")))))

(event EventBeginPlay
  (bind _asversion_2_gm (Utilities|Casting|CastToVersion2_GM (Game|GetGameMode)))
  (Variables|Default|SetMyGameMode _asversion_2_gm)
  (bind _asenemy_health_bar (Utilities|Casting|CastToEnemyHealthBar (UserInterface|GetUserWidgetObject (Variables|Default|GetHealthBar))))
  (Variables|Default|SetMyHealthBar _asenemy_health_bar)
  (bind _returnvalue (Sequencer|Player|CreateLevelSequencePlayer (Variables|Default|GetSequencer)))
  (Variables|Default|SetSequencerPlayer _returnvalue))

(event Game|Damage|EventAnyDamage
  (params (Damage :type Float%20%28single-precision%29) (DamageType :type Damage%20Type%20Object%20Reference) (InstigatedBy :type Controller%20Object%20Reference) (DamageCauser :type Actor%20Object%20Reference))
  (Development|PrintString (Utilities|String|ToString(Float) Damage))
  (Variables|State|SetHealth (- (Variables|State|GetHealth) (/ Damage (Variables|State|GetDEF))))
  (Default|SetPercentage (Variables|Default|GetMyHealthBar) (/ (Variables|State|GetHealth) (Variables|State|GetMaxHealth)))
  (if (<= (Variables|State|GetHealth) 0.0)
    (Default|Win (Variables|Default|GetMyGameMode))))

(fn ConstructionScript)