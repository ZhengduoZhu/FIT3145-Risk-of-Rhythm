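; Rhythm-game spawner and judge for two lanes, up and down, creating BP_Beat notes at each lane's spawn point tagged with their direction.
; Nested Perfect, Great and Good overlap volumes per lane update each beat's Credit as it enters and leaves, ending in Miss.
; The Good volumes also add and remove beats in the Version2_GM game mode's per-lane note lists.
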(event OnComponentBeginOverlap(Perfect_U)
  (params (OverlappedComponent :type Primitive%20Component%20Object%20Reference) (OtherActor :type Actor%20Object%20Reference) (OtherComp :type Primitive%20Component%20Object%20Reference) (OtherBodyIndex :type Integer) (bFromSweep :type Boolean) (SweepResult :type Hit%20Result%20Structure%20%28by%20ref%29))
  (bind _asbp_beat (Utilities|Casting|CastToBP_Beat OtherActor))
  (Variables|/Game/ZhengduoZhu/Blueprint/BP_Beat.BP_Beat_C|SetCredit _asbp_beat "Perfect"))

(event OnComponentEndOverlap(Perfect_U)
  (params (OverlappedComponent :type Primitive%20Component%20Object%20Reference) (OtherActor :type Actor%20Object%20Reference) (OtherComp :type Primitive%20Component%20Object%20Reference) (OtherBodyIndex :type Integer))
  (bind _asbp_beat (Utilities|Casting|CastToBP_Beat OtherActor))
  (Variables|/Game/ZhengduoZhu/Blueprint/BP_Beat.BP_Beat_C|SetCredit _asbp_beat "Great"))

(event OnComponentBeginOverlap(Good_D)
  (params (OverlappedComponent :type Primitive%20Component%20Object%20Reference) (OtherActor :type Actor%20Object%20Reference) (OtherComp :type Primitive%20Component%20Object%20Reference) (OtherBodyIndex :type Integer) (bFromSweep :type Boolean) (SweepResult :type Hit%20Result%20Structure%20%28by%20ref%29))
  (bind _asbp_beat (Utilities|Casting|CastToBP_Beat OtherActor))
  (Utilities|Array|Add (Variables|/Game/ZhengduoZhu/Blueprint/Version2/Version2_GM.Version2_GM_C|GetNotes2 (Variables|Default|GetMyGameMode)) _asbp_beat)
  (Variables|/Game/ZhengduoZhu/Blueprint/BP_Beat.BP_Beat_C|SetCredit _asbp_beat "Good"))

(event OnComponentEndOverlap(Good_D)
  (params (OverlappedComponent :type Primitive%20Component%20Object%20Reference) (OtherActor :type Actor%20Object%20Reference) (OtherComp :type Primitive%20Component%20Object%20Reference) (OtherBodyIndex :type Integer))
  (bind _asbp_beat (Utilities|Casting|CastToBP_Beat OtherActor))
  (Utilities|Array|RemoveItem (Variables|/Game/ZhengduoZhu/Blueprint/Version2/Version2_GM.Version2_GM_C|GetNotes2 (Variables|Default|GetMyGameMode)) _asbp_beat)
  (Variables|/Game/ZhengduoZhu/Blueprint/BP_Beat.BP_Beat_C|SetCredit _asbp_beat "Miss"))

(event OnComponentBeginOverlap(Great_U)
  (params (OverlappedComponent :type Primitive%20Component%20Object%20Reference) (OtherActor :type Actor%20Object%20Reference) (OtherComp :type Primitive%20Component%20Object%20Reference) (OtherBodyIndex :type Integer) (bFromSweep :type Boolean) (SweepResult :type Hit%20Result%20Structure%20%28by%20ref%29))
  (bind _asbp_beat (Utilities|Casting|CastToBP_Beat OtherActor))
  (Variables|/Game/ZhengduoZhu/Blueprint/BP_Beat.BP_Beat_C|SetCredit _asbp_beat "Great"))

(event OnComponentEndOverlap(Great_U)
  (params (OverlappedComponent :type Primitive%20Component%20Object%20Reference) (OtherActor :type Actor%20Object%20Reference) (OtherComp :type Primitive%20Component%20Object%20Reference) (OtherBodyIndex :type Integer))
  (bind _asbp_beat (Utilities|Casting|CastToBP_Beat OtherActor))
  (Variables|/Game/ZhengduoZhu/Blueprint/BP_Beat.BP_Beat_C|SetCredit _asbp_beat "Good"))

(event OnComponentBeginOverlap(Good_U)
  (params (OverlappedComponent :type Primitive%20Component%20Object%20Reference) (OtherActor :type Actor%20Object%20Reference) (OtherComp :type Primitive%20Component%20Object%20Reference) (OtherBodyIndex :type Integer) (bFromSweep :type Boolean) (SweepResult :type Hit%20Result%20Structure%20%28by%20ref%29))
  (bind _asbp_beat (Utilities|Casting|CastToBP_Beat OtherActor))
  (Utilities|Array|Add (Variables|/Game/ZhengduoZhu/Blueprint/Version2/Version2_GM.Version2_GM_C|GetNotes1 (Variables|Default|GetMyGameMode)) _asbp_beat)
  (Variables|/Game/ZhengduoZhu/Blueprint/BP_Beat.BP_Beat_C|SetCredit _asbp_beat "Good"))

(event OnComponentEndOverlap(Good_U)
  (params (OverlappedComponent :type Primitive%20Component%20Object%20Reference) (OtherActor :type Actor%20Object%20Reference) (OtherComp :type Primitive%20Component%20Object%20Reference) (OtherBodyIndex :type Integer))
  (bind _asbp_beat (Utilities|Casting|CastToBP_Beat OtherActor))
  (Utilities|Array|RemoveItem (Variables|/Game/ZhengduoZhu/Blueprint/Version2/Version2_GM.Version2_GM_C|GetNotes1 (Variables|Default|GetMyGameMode)) _asbp_beat)
  (Variables|/Game/ZhengduoZhu/Blueprint/BP_Beat.BP_Beat_C|SetCredit _asbp_beat "Miss"))

(event OnComponentBeginOverlap(Perfect_D)
  (params (OverlappedComponent :type Primitive%20Component%20Object%20Reference) (OtherActor :type Actor%20Object%20Reference) (OtherComp :type Primitive%20Component%20Object%20Reference) (OtherBodyIndex :type Integer) (bFromSweep :type Boolean) (SweepResult :type Hit%20Result%20Structure%20%28by%20ref%29))
  (bind _asbp_beat (Utilities|Casting|CastToBP_Beat OtherActor))
  (Variables|/Game/ZhengduoZhu/Blueprint/BP_Beat.BP_Beat_C|SetCredit _asbp_beat "Perfect"))

(event OnComponentEndOverlap(Perfect_D)
  (params (OverlappedComponent :type Primitive%20Component%20Object%20Reference) (OtherActor :type Actor%20Object%20Reference) (OtherComp :type Primitive%20Component%20Object%20Reference) (OtherBodyIndex :type Integer))
  (bind _asbp_beat (Utilities|Casting|CastToBP_Beat OtherActor))
  (Variables|/Game/ZhengduoZhu/Blueprint/BP_Beat.BP_Beat_C|SetCredit _asbp_beat "Great"))

(event OnComponentBeginOverlap(Great_D)
  (params (OverlappedComponent :type Primitive%20Component%20Object%20Reference) (OtherActor :type Actor%20Object%20Reference) (OtherComp :type Primitive%20Component%20Object%20Reference) (OtherBodyIndex :type Integer) (bFromSweep :type Boolean) (SweepResult :type Hit%20Result%20Structure%20%28by%20ref%29))
  (bind _asbp_beat (Utilities|Casting|CastToBP_Beat OtherActor))
  (Variables|/Game/ZhengduoZhu/Blueprint/BP_Beat.BP_Beat_C|SetCredit _asbp_beat "Great"))

(event OnComponentEndOverlap(Great_D)
  (params (OverlappedComponent :type Primitive%20Component%20Object%20Reference) (OtherActor :type Actor%20Object%20Reference) (OtherComp :type Primitive%20Component%20Object%20Reference) (OtherBodyIndex :type Integer))
  (bind _asbp_beat (Utilities|Casting|CastToBP_Beat OtherActor))
  (Variables|/Game/ZhengduoZhu/Blueprint/BP_Beat.BP_Beat_C|SetCredit _asbp_beat "Good"))

(event Custom|SpawnBeat_U
  (bind _spawnpoint_u (Variables|Default|GetSpawnPoint_U))
  (bind _returnvalue (Transformation|GetWorldTransform _spawnpoint_u))
  (bind _returnvalue_2 (Game|SpawnActorfromClass "/Game/ZhengduoZhu/Blueprint/BP_Beat.BP_Beat_C" (Math|Transform|MakeTransform (.location _returnvalue) (.rotation _returnvalue) "0.100000,0.100000,0.100000") "Undefined" 0 0))
  (Variables|/Game/ZhengduoZhu/Blueprint/BP_Beat.BP_Beat_C|SetDirection _returnvalue_2 "UP"))

(event Custom|SpawnBeat_D
  (bind _spawnpoint_d (Variables|Default|GetSpawnPoint_D))
  (bind _returnvalue (Transformation|GetWorldTransform _spawnpoint_d))
  (bind _returnvalue_2 (Game|SpawnActorfromClass "/Game/ZhengduoZhu/Blueprint/BP_Beat.BP_Beat_C" (Math|Transform|MakeTransform (.location _returnvalue) (.rotation _returnvalue) "0.100000,0.100000,0.100000") "Undefined" 0 0))
  (Variables|/Game/ZhengduoZhu/Blueprint/BP_Beat.BP_Beat_C|SetDirection _returnvalue_2 "DOWN"))

(event EventBeginPlay
  (bind _asversion_2_gm (Utilities|Casting|CastToVersion2_GM (Game|GetGameMode)))
  (Variables|Default|SetMyGameMode _asversion_2_gm))

(event Collision|EventActorBeginOverlap
  (params (OtherActor :type Actor%20Object%20Reference)))

(event EventTick
  (params (DeltaSeconds :type Float%20%28single-precision%29)))

(fn ConstructionScript)