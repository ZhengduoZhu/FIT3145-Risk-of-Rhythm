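; Game manager for a rhythm-based battle mode, where hitting notes in an up and a down lane deals the player's attack as damage.
; StartBattle repositions the character, switches to battle mode, fades to a fixed battle camera, shows the HUD and plays a level sequence after a countdown.
; Tick targets each lane's first note, which player input breaks, spawning credit-based combo UI and a hit sound.
; Win pauses the game.
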(event Custom|StartBattle
  (params (Monster :type BP%20Monster%20Version%202%20Object%20Reference))
  (bind _mycharacter (Variables|Default|GetMyCharacter))
  (Variables|Default|SetBattleStart true)
  (Transformation|SetActorTransform _mycharacter (Math|Transform|MakeTransform "-676.000000,9138.000000,23.000000" "0,90.000000, 0" "1,1,1"))
  (Components|Movement|StopMovementImmediately (Variables|/Script/Engine.Character|GetCharacterMovement _mycharacter))
  (Variables|Default|SetMyMonster Monster)
  (Variables|/Game/ZhengduoZhu/Blueprint/PC_Zheng.PC_Zheng_C|SetBattleMode (Variables|Default|GetMyPlayerController) true)
  (Default|ActiviteSkills (Variables|Default|GetMyCharacter))
  (Variables|/Game/ZhengduoZhu/Character/Version2_Character.Version2_Character_C|SetBattleMode (Variables|Default|GetMyCharacter) true)
  (Variables|/Script/Engine.PlayerController|SetbShowMouseCursor (Game|GetPlayerController 0) false)
  (CameraFades|StartCameraFade :self (Game|GetPlayerCameraManager 0) :ToAlpha 1.0 :Duration 1.0 :bHoldWhenFinished true)
  (Utilities|FlowControl|Delay 1.0)
  (Game|Player|SetViewTargetwithBlend (Game|GetPlayerController 0) (Variables|Default|GetBattleCamera) 0.0 "VTBlend_EaseInOut" 0.0 false)
  (CameraFades|StartCameraFade :self (Game|GetPlayerCameraManager 0) :FromAlpha 1.0 :Duration 1.0 :bHoldWhenFinished true)
  (bind _returnvalue (UserInterface|CreateWidget "/Game/ZhengduoZhu/UI/PlayerManaBar.PlayerManaBar_C" (Variables|Default|GetMyPlayerController)))
  (UserInterface|Viewport|AddtoViewport _returnvalue 0)
  (bind _returnvalue_2 (UserInterface|CreateWidget "/Game/ZhengduoZhu/UI/CountDownUI.CountDownUI_C" (Variables|Default|GetMyPlayerController)))
  (UserInterface|Viewport|AddtoViewport _returnvalue_2 0)
  (bind _returnvalue_3 (UserInterface|CreateWidget "/Game/Nicolas/UI/SongDetails.SongDetails_C" (Variables|Default|GetMyPlayerController)))
  (UserInterface|Viewport|AddtoViewport _returnvalue_3 0)
  (Utilities|FlowControl|Delay 5.0)
  (Widget|RemovefromParent _returnvalue_2)
  (Sequencer|Player|Play (Variables|Default|GetSequencer) :!class /Script/MovieScene.MovieSceneSequencePlayer)
  (Utilities|Time|SetGlobalTimeDilation 1.0))

(event Custom|ReceiveInput
  (params (Input :type String))
  (bind _mycharacter (Variables|Default|GetMyCharacter))
  (bind _uptarget (Variables|Default|GetUpTarget))
  (bind _downtarget (Variables|Default|GetDownTarget))
  (bind _credit (Variables|/Game/ZhengduoZhu/Blueprint/BP_Beat.BP_Beat_C|GetCredit _downtarget))
  (bind _credit_2 (Variables|/Game/ZhengduoZhu/Blueprint/BP_Beat.BP_Beat_C|GetCredit _uptarget))
  (bind _atk (Variables|/Game/ZhengduoZhu/Character/Version2_Character.Version2_Character_C|GetATK _mycharacter))
  ;[1 1 1] DetectInput
  (switch string Input
    (:UP
      (Utilities|IsValid (Variables|Default|GetUpTarget)
        (:Is%20Valid
          (Variables|Default|SetValidUpInput true)
          (Variables|/Game/ZhengduoZhu/Blueprint/BP_Beat.BP_Beat_C|SetDamage _uptarget _atk)
          (CallFunction|CreateComboUI _credit_2)
          (CallFunction|CreateSound _credit_2)
          (Default|BreakBeat _uptarget)
          (Utilities|Array|RemoveItem (Variables|Default|GetNotes1) (Variables|Default|GetUpTarget))
          (Variables|Default|SetValidUpInput false))))
    (:DOWN
      (Utilities|IsValid (Variables|Default|GetDownTarget)
        (:Is%20Valid
          (Variables|Default|SetValidDownInput true)
          (Variables|/Game/ZhengduoZhu/Blueprint/BP_Beat.BP_Beat_C|SetDamage _downtarget _atk)
          (CallFunction|CreateComboUI _credit)
          (CallFunction|CreateSound _credit)
          (Default|BreakBeat _downtarget)
          (Utilities|Array|RemoveItem (Variables|Default|GetNotes2) (Variables|Default|GetDownTarget))
          (Variables|Default|SetValidDownInput false))))))

(event Custom|CreateComboUI
  (params (Input :type String))
  ;[1 1 1] Create Combo UI
  (bind _returnvalue (UserInterface|CreateWidget "/Game/ZhengduoZhu/UI/ComboWidget.ComboWidget_C" (Variables|Default|GetMyPlayerController)))
  (Default|SetComboText _returnvalue (Utilities|Text|ToText(String) Input))
  (UserInterface|Viewport|AddtoViewport _returnvalue 0))

(event Custom|Win
  (Game|SetGamePaused true))

(event Custom|CreateSound
  (params (Credit :type String))
  (switch string Credit
    (:Great
      (Audio|PlaySound2D "/Game/Swords_Sounds_Pro/Wavs/Sword_hit_shield/Sword_hit_shield_4.Sword_hit_shield_4" 1.0 1.0 0.0 0 0))
    (:Good
      (Audio|PlaySound2D "/Game/Swords_Sounds_Pro/Wavs/Sword_hit_shield/Sword_hit_shield_4.Sword_hit_shield_4" 1.0 1.0 0.0 0 0))
    (:Perfect
      (Audio|PlaySound2D "/Game/Swords_Sounds_Pro/Wavs/Sword_hit_shield/Sword_hit_shield_4.Sword_hit_shield_4" 1.0 1.0 0.0 0 0))))

(event EventBeginPlay
  (Variables|Default|SetBattleCamera (Components|GetOwner (Variables|Default|GetCamera)))
  (bind _aspc_zheng (Utilities|Casting|CastToPC_Zheng (Game|GetPlayerController 0)))
  (bind _output_get (Variables|Default|SetMyPlayerController _aspc_zheng))
  (bind _asversion_2_character (Utilities|Casting|CastToVersion2_Character (Pawn|GetControlledPawn _output_get)))
  (Variables|Default|SetMyCharacter _asversion_2_character)
  (Transformation|SetActorTransform (Variables|Default|GetBattleCamera) (Math|Transform|MakeTransform "-1150.000000,9515.000000,250.000000" "0, 0, 0" "1,1,1"))
  (bind _returnvalue (Sequencer|Player|CreateLevelSequencePlayer "/Game/General/Squencer/effectedByJeffrey/newVerSeq/whatThisCouldBeHardOffset.whatThisCouldBeHardOffset"))
  (Variables|Default|SetSequencer _returnvalue))

(event EventTick
  (params (DeltaSeconds :type Float%20%28single-precision%29))
  ;[1 1 1] SetTarget
  (Utilities|FlowControl|Sequence
    (:then_0
      (if (!= (Utilities|Array|Length (Variables|Default|GetNotes1)) 0)
        (Variables|Default|SetUpTarget (Utilities|Array|Get(acopy) (Variables|Default|GetNotes1)))
        (goto _label Reset)
        (else
          (Utilities|FlowControl|DoOnce false :!label _label
            (:Completed
              (Variables|Default|SetUpTarget 0))))))
    (:then_1
      (if (!= (Utilities|Array|Length (Variables|Default|GetNotes2)) 0)
        (Variables|Default|SetDownTarget (Utilities|Array|Get(acopy) (Variables|Default|GetNotes2)))
        (goto _label_2 Reset)
        (else
          (Utilities|FlowControl|DoOnce false :!label _label_2
            (:Completed
              (Variables|Default|SetDownTarget 0))))))))

(fn ConstructionScript)